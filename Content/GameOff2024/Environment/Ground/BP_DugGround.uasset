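; BP_DugGround is a dug ground environment piece that reveals itself in stages.
; The construction script hides DigPile and its child components.
; RevealDugGround runs once, activating DigEffect and showing three stage components in sequence, spaced by delays of a third of the given duration.
; After the final delay, it pauses and destroys the effect, leaving the revealed stages visible.
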(event `RevealDugGround`
  (params (Duration :type "Float (double-precision)" :default 1.0))
  (bind _digeffect (`self.DigEffect`))
  (if (not (`self.IsRevealed`))
    (set `self.IsRevealed` true)
    (`ActorComponent.Activate` (`self.DigEffect`) false)
    (bind _output_get (set `self.StageDuration` (/ Duration 3.0)))
    (`SceneComponent.SetVisibility` (`self.Stage1`) true true)
    (`KismetSystemLibrary.Delay` _output_get)
    (`SceneComponent.SetVisibility` (`self.Stage2`) true true)
    (`KismetSystemLibrary.Delay` _output_get)
    (`SceneComponent.SetVisibility` (`self.Stage3`) true true)
    (`KismetSystemLibrary.Delay` _output_get)
    (`NiagaraComponent.SetPaused` _digeffect true)
    (`ActorComponent.K2_DestroyComponent` _digeffect)))

(fn `UserConstructionScript`
  (`SceneComponent.SetVisibility` (`self.DigPile`) false true))