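; BP_HoleMesh is a ground environment actor that defines an oriented volume for a dissolve effect, apparently to cut a hole.
; Its construction script writes the InclusionBounds component's world location, scale and forward, right and up axes into the MPC_Dissolve material parameter collection.
; The collection is global and only written during construction, so each instance overwrites the same values and runtime movement is not tracked.
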(fn `UserConstructionScript`
  (bind _inclusionbounds (`self.InclusionBounds`))
  (`KismetMaterialLibrary.SetVectorParameterValue` "/Game/GameOff2024/Environment/Ground/MPC_Dissolve.MPC_Dissolve" "Location" (`KismetMathLibrary.Conv_VectorToLinearColor` (`SceneComponent.K2_GetComponentLocation` (`self.InclusionBounds`))))
  (`KismetMaterialLibrary.SetVectorParameterValue` "/Game/GameOff2024/Environment/Ground/MPC_Dissolve.MPC_Dissolve" "Effect Size" (`KismetMathLibrary.Conv_VectorToLinearColor` (`SceneComponent.K2_GetComponentScale` (`self.InclusionBounds`))))
  (`KismetMaterialLibrary.SetVectorParameterValue` "/Game/GameOff2024/Environment/Ground/MPC_Dissolve.MPC_Dissolve" "X" (`KismetMathLibrary.Conv_VectorToLinearColor` (`SceneComponent.GetForwardVector` _inclusionbounds)))
  (`KismetMaterialLibrary.SetVectorParameterValue` "/Game/GameOff2024/Environment/Ground/MPC_Dissolve.MPC_Dissolve" "Y" (`KismetMathLibrary.Conv_VectorToLinearColor` (`SceneComponent.GetRightVector` _inclusionbounds)))
  (`KismetMaterialLibrary.SetVectorParameterValue` "/Game/GameOff2024/Environment/Ground/MPC_Dissolve.MPC_Dissolve" "Z" (`KismetMathLibrary.Conv_VectorToLinearColor` (`SceneComponent.GetUpVector` _inclusionbounds))))