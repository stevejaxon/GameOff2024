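; BP_Hex_City is the city hex tile for the game's tile grid.
; It extends a parent tile, adding cursor-hover handling that shows and hides a highlight feedback widget.
; Clicking it triggers the invalid-selection response, and releasing the click is deliberately left empty.
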(event `self.ReceiveActorBeginCursorOver`
  (`parent.ReceiveActorBeginCursorOver`)
  (`SceneComponent.SetVisibility` (`self.TileHighlightedFeedbackWidgetComp`) true false))

(event `self.ReceiveActorEndCursorOver`
  (`parent.ReceiveActorEndCursorOver`)
  (`SceneComponent.SetVisibility` (`self.TileHighlightedFeedbackWidgetComp`) false false))

(event `self.ReceiveActorOnClicked`
  (params (ButtonPressed :type "Key Structure"))
  (`self.On Invalid Selection`))

(event `self.ReceiveActorOnReleased`
  (params (ButtonReleased :type "Key Structure"))
  ;[1 1 1] Do nothing
)

(fn `UserConstructionScript`
  (`parent.UserConstructionScript`))