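; Interactive hexagonal tile with PCG-generated content that responds to cursor hover, click selection and highlight feedback.
; Hover timelines lift and scale the tile, while cursor handlers pass its notify pattern and distance for highlighting.
; Pressing drives a material progress fill that reverses on release; its finish reports the tile index to MainGameModeBase.
; Negative highlights and the invalid-selection shake temporarily hide the PCG components.
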(event OnPCGGraphGeneratedExternal(PCG)
  (params (PCGComponent :type PCG%20Component%20Object%20Reference))
  (Class|TileBase|HandlePGCGenerationCompleted))

(event Custom|On%20Invalid%20Selection
  (Class|TileBase|HidePCGComponents)
  (bind _shake (Timeline|Invalid%20Selection%20Feedback PlayFromStart)
    (:Update
      (UX|AnimateInvalidSelection _shake))
    (:Finished
      (Class|TileBase|ShowPCGComponents))))

(event EventOnHighlightTileStart
  (params (HoveredTileType :type UETileType%20Enum :default "None") (Feedback :type ETileInteractionFeedback%20Enum :default "None") (FeedbackColor :type Linear%20Color%20Structure))
  (CallFunction|UpdateMIDS FeedbackColor FeedbackColor)
  (if (Utilities|Enum|Equal(Enum) Feedback "Positive")
    (Rendering|SetVisibility (Variables|Default|GetTileHighlightedWidgetComp) true false)
    (else
      (Rendering|SetVisibility (Variables|Default|GetTileHighlightedWidgetComp) true false)
      (Class|TileBase|HidePCGComponents)
      (Rendering|SetVisibility (Variables|Default|GetTileHighlightedFeedbackWidgetComp) true false))))

(event MouseInput|EventActorOnClicked
  (params (ButtonPressed :type Key%20Structure :default "None"))
  (if (not (Variables|UI|GetIsSelected))
    (Rendering|SetVisibility (Variables|Default|GetTileSelectedWidgetComp) true false)
    (bind _progress (Timeline|SelectedProgress Play)
      (:Update
        (Rendering|Material|SetScalarParameterValue (UserInterface|GetMaterialInstance (Variables|Default|GetTileSelectedWidgetComp)) "ProgressAmount" _progress :!class /Script/Engine.MaterialInstanceDynamic))
      (:Finished
        (CallFunction|HandleSelectionAnimFinished _progress)
        (bind _asmain_game_mode_base (Utilities|Casting|CastToMainGameModeBase (Game|GetGameMode)))
        (Class|MainGameModeBase|TileSelected _asmain_game_mode_base (Variables|Default|GetTileIndex))))))

(event MouseInput|EventActorBeginCursorOver
  (bind _uxfeedbackcolor (Variables|Default|GetUXFeedbackColor))
  (CallFunction|UpdateMIDS _uxfeedbackcolor _uxfeedbackcolor)
  (Rendering|SetVisibility (Variables|Default|GetTileHighlightedWidgetComp) true false)
  (Class|TileBase|HandleTileCursorOverBegin (Variables|UX|GetNotify%20Pattern) (Variables|UX|GetFeedback) (Variables|Default|GetUXFeedbackColor) (Variables|UX|GetNotify%20Distance))
  (if (Variables|Default|GetCanScale)
    (Variables|Default|SetCanScale false)
    (bind (_direction _scale_up_on_hover_over _lift_up_on_hover_over) (Timeline|CursorOverAnimation PlayFromStart)
      (:Update
        (UX|AnimateTile _scale_up_on_hover_over _lift_up_on_hover_over)))))

(event EventOnHighlightTileEnd
  (Rendering|SetVisibility (Variables|Default|GetTileHighlightedWidgetComp) false false)
  (Rendering|SetVisibility (Variables|Default|GetTileHighlightedFeedbackWidgetComp) false false)
  (Class|TileBase|ShowPCGComponents))

(event MouseInput|EventActorEndCursorOver
  (Rendering|SetVisibility (Variables|Default|GetTileHighlightedWidgetComp) false false)
  (Class|TileBase|HandleTileCursorOverEnd (Variables|UX|GetNotify%20Pattern) (Variables|UX|GetNotify%20Distance))
  (bind (_direction _scale_down_on_hover_left _move_downwards_on_hover_left) (Timeline|CursorLeftAnimation PlayFromStart)
    (:Update
      (UX|AnimateTile _scale_down_on_hover_left _move_downwards_on_hover_left))
    (:Finished
      (Variables|Default|SetCanScale true))))

(event EventActorOnReleased
  (params (ButtonReleased :type Key%20Structure :default "None"))
  (if (not (Variables|UI|GetIsSelected))
    (bind _progress (Timeline|SelectedProgress Reverse)
      (:Update
        (Rendering|Material|SetScalarParameterValue (UserInterface|GetMaterialInstance (Variables|Default|GetTileSelectedWidgetComp)) "ProgressAmount" _progress :!class /Script/Engine.MaterialInstanceDynamic))
      (:Finished
        (CallFunction|HandleSelectionAnimFinished _progress)
        (bind _asmain_game_mode_base (Utilities|Casting|CastToMainGameModeBase (Game|GetGameMode)))
        (Class|MainGameModeBase|TileSelected _asmain_game_mode_base (Variables|Default|GetTileIndex))))))

(fn ConstructionScript
  (bind _rootcomponent (Variables|Transformation|GetRootComponent))
  (bind _returnvalue (Transformation|GetWorldLocation _rootcomponent))
  (Class|PCGComponent|SetGraph (Variables|Default|GetPCG) (Variables|PCG|GetPCGGraph))
  (Variables|PCG|SetPCGTileCenter _returnvalue)
  (Variables|Default|SetOriginal%20Location _returnvalue)
  (Variables|PCG|SetPCGRandSeed (Class|KismetMathLibrary|RandomIntegerfromStream (Math|Random|MakeRandomStream (Math|Float|Truncate (.X (Math|Vector|BreakVector _returnvalue)))) 2147483646))
  (Transformation|SetRelativeLocation (Variables|Default|GetTileHighlightedWidgetComp) (Math|Vector|MakeVector 0.0 0.0 (Variables|UI|GetUIWidgetOffset)) false false)
  (Transformation|SetRelativeLocation (Variables|Default|GetTileSelectedWidgetComp) (Math|Vector|MakeVector 0.0 0.0 (+ (Variables|UI|GetUIWidgetOffset) 0.1)) false false)
  (Transformation|SetRelativeLocation (Variables|Default|GetTileHighlightedFeedbackWidgetComp) (Math|Vector|MakeVector 0.0 0.0 (Variables|UI|GetUIWidgetOffset)) false false))

(fn UpdateMIDS
  (params (Highlight%20Color :type Linear%20Color%20Structure) (Feedback%20Color :type Linear%20Color%20Structure))
  (if (Variables|Default|GetMIDsInitialized)
    (return)
    (else
      (Utilities|FlowControl|Sequence
        (:then_0
          (Rendering|Material|SetVectorParameterValue (UserInterface|GetMaterialInstance (Variables|Default|GetTileHighlightedWidgetComp)) "FillColor" Highlight%20Color :!class /Script/Engine.MaterialInstanceDynamic))
        (:then_1
          (Rendering|Material|SetVectorParameterValue (UserInterface|GetMaterialInstance (Variables|Default|GetTileHighlightedFeedbackWidgetComp)) "FillColor" Feedback%20Color :!class /Script/Engine.MaterialInstanceDynamic)
          (return))))))

(fn HandleSelectionAnimFinished
  (params (A :type Float%20%28double-precision%29))
  (Rendering|SetVisibility (Variables|Default|GetTileSelectedWidgetComp) false false)
  (if (== A 1.0)
    (Variables|UI|SetIsSelected true)))

(fn UpdateTileScale
  (params (ScaleIncrement :type Float%20%28double-precision%29))
  (return (Math|Conversions|ToVector(Float) (+ (* ScaleIncrement (Variables|UX|GetTargetScale)) (Variables|Default|GetOriginalScale)))))

(fn AnimateTile
  (params (ScaleIncrement :type Float%20%28double-precision%29) (LocationIncrement :type Float%20%28double-precision%29))
  (bind _original_location (Variables|Default|GetOriginal%20Location))
  (bind _newscale (UX|UpdateTileScale ScaleIncrement))
  (Transformation|SetWorldTransform (Variables|Transformation|GetRootComponent) (Math|Transform|MakeTransform (Math|Vector|MakeVector (.x _original_location) (.y _original_location) (+ (.z _original_location) (* LocationIncrement (Variables|UX|GetTargetHeight)))) "0, 0, 0" _newscale) false false)
  (return))

(fn AnimateInvalidSelection
  (params (A :type Float%20%28double-precision%29))
  (bind _original_location (Variables|Default|GetOriginal%20Location))
  (Transformation|SetWorldLocation (Variables|Transformation|GetRootComponent) (Math|Vector|MakeVector (.x _original_location) (+ (.y _original_location) (* A (Variables|UX|GetHorizontalFeedbackAmount))) (Variables|UX|GetTargetHeight)) false false))