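; Main game mode that runs the tile-reveal flow and creates the HUD with mouse click and hover input.
; Selecting a tile locks click and hover, moves a switchable camera there, blends to it, then broadcasts the reveal.
; Once revealed, the view blends back to the pawn, input returns and a goal tile enables the HUD button.
; The game instance's level-loaded transition fires from both construction and BeginPlay.
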(event `self.ReceiveBeginPlay`
  (bind _returnvalue (`GameplayStatics.GetPlayerController` 0))
  (set `PlayerController.bShowMouseCursor` true _returnvalue)
  (set `PlayerController.bEnableMouseOverEvents` true _returnvalue)
  (set `PlayerController.bEnableClickEvents` true _returnvalue)
  (bind _returnvalue_2 (`|CreateWidget` "/Game/GameOff2024/UI/Level/WBP_UI_HUD.WBP_UI_HUD_C"))
  (bind _output_get (set `self.HUD UI` _returnvalue_2))
  (`UserWidget.AddToViewport` _output_get 0)
  (`/Game/GameOff2024/Core/GameModes/BP_Main_GI.StartLevelLoadedTransition` (`self.MainGI`))
  (`|ExecutionSequence`
    (:`then_0`
      (bind _asbp_main_pawn (cast `/Game/GameOff2024/Core/Player/BP_MainPawn` (`GameplayStatics.GetPlayerPawn` 0)))
      (set `self.Main Pawn` _asbp_main_pawn))
    (:`then_1`
      (bind _returnvalue_3 (`GameplayStatics.GetActorOfClass` "/Game/GameOff2024/Core/Player/BP_SwitchableCamera.BP_SwitchableCamera_C"))
      (set `self.ZoomedInCamera` _returnvalue_3))))

(event `self.TileSelected`
  (params (SelectedTileIndex :type Integer) (TileLocation :type "Vector Structure"))
  (bind _returnvalue (`GameplayStatics.GetPlayerController` 0))
  (bind _camera_zoom_time (`self.Camera Zoom Time`))
  (set `PlayerController.bEnableMouseOverEvents` false _returnvalue)
  (set `PlayerController.bEnableClickEvents` false _returnvalue)
  (`SceneComponent.K2_SetWorldLocation` (`/Game/GameOff2024/Core/Player/BP_SwitchableCamera.DefaultSceneRoot` (`self.ZoomedInCamera`)) TileLocation false true)
  (`PlayerController.SetViewTargetWithBlend` (`GameplayStatics.GetPlayerController` 0) (`self.ZoomedInCamera`) _camera_zoom_time "VTBlend_Linear" 0.0 false)
  (`KismetSystemLibrary.Delay` _camera_zoom_time)
  (`self.OnRevealTileContents` SelectedTileIndex))

(event `self.SelectedTilesContentsRevealed`
  (params (SelectedTileIndex :type Integer))
  (bind _returnvalue (`GameplayStatics.GetPlayerController` 0))
  (bind _camera_zoom_time (`self.Camera Zoom Time`))
  (`PlayerController.SetViewTargetWithBlend` _returnvalue (`self.Main Pawn`) _camera_zoom_time "VTBlend_Linear" 0.0 false)
  (`KismetSystemLibrary.Delay` _camera_zoom_time)
  (set `PlayerController.bShowMouseCursor` true _returnvalue)
  (set `PlayerController.bEnableMouseOverEvents` true _returnvalue)
  (set `PlayerController.bEnableClickEvents` true _returnvalue)
  (bind _returnvalue_2 (`self.IsGoalLocation` SelectedTileIndex))
  (if _returnvalue_2
    (`/Game/GameOff2024/UI/Level/WBP_UI_HUD.Enable Button` (`self.HUD UI`))))

(fn `UserConstructionScript`
  (bind _asbp_main_gi (cast `/Game/GameOff2024/Core/GameModes/BP_Main_GI` (`GameplayStatics.GetGameInstance`)))
  (bind _output_get (set `self.MainGI` _asbp_main_gi))
  (`/Game/GameOff2024/Core/GameModes/BP_Main_GI.StartLevelLoadedTransition` _output_get))