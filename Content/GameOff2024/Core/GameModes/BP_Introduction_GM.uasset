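; BP_Introduction_GM is the game mode for the game's introduction screen.
; On BeginPlay it creates and shows the WBP_UI_Introduction widget, triggers the level-loaded transition on BP_Main_GI, and shows the mouse cursor.
; The construction script caches the game instance cast, and StartIntroduction passes its data on to the widget's Start function.
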(event `self.ReceiveBeginPlay`
  (bind _returnvalue (`|CreateWidget` "/Game/GameOff2024/UI/Tutorial/WBP_UI_Introduction.WBP_UI_Introduction_C"))
  (bind _output_get (set `self.IntroductionUI` _returnvalue))
  (`UserWidget.AddToViewport` _output_get 0)
  (`/Game/GameOff2024/Core/GameModes/BP_Main_GI.StartLevelLoadedTransition` (`self.Main GI`))
  (set `PlayerController.bShowMouseCursor` true (`GameplayStatics.GetPlayerController` 0)))

(fn `StartIntroduction`
  (params (Data :type "Array of /Game/GameOff2024/UI/Tutorial/TutorialDataStruct Structure"))
  (`/Game/GameOff2024/UI/Tutorial/WBP_UI_Introduction.Start` (`self.IntroductionUI`) Data))

(fn `UserConstructionScript`
  (bind _asbp_main_gi (cast `/Game/GameOff2024/Core/GameModes/BP_Main_GI` (`GameplayStatics.GetGameInstance`)))
  (set `self.Main GI` _asbp_main_gi))