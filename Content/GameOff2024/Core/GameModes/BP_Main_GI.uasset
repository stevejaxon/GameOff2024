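; Game instance that owns the screen transition widget used when moving between levels.
; Init creates one UI_Transition widget, which the transition functions add to the viewport if needed before starting their load-out or level-loaded animation.
; OpenNewLevel starts the outgoing transition, and its completion event then calls LoadNextLevel with the level name.
; The level-loaded completion event is an empty stub.
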(event `Add Loading UI`
  (`UserWidget.AddToViewport` (`self.UI Transition Widget`) 0))

(event `Open New Level`
  (params (LevelName :type Name))
  (`self.StartLoadNewLevelTransition` LevelName))

(event `self.ReceiveInit`
  (bind _returnvalue (`|CreateWidget` "/Game/GameOff2024/UI/UI_Transition.UI_Transition_C"))
  (set `self.UI Transition Widget` _returnvalue))

(event `New Level Loaded Transition Complete`)

(event `Load New Level Transition Complete`
  (params (LevelName :type Name))
  (`self.LoadNextLevel` LevelName))

(fn `StartLevelLoadedTransition`
  (bind _ui_transition_widget (`self.UI Transition Widget`))
  (if (not (`Widget.IsInViewport` _ui_transition_widget))
    (`UserWidget.AddToViewport` _ui_transition_widget 0))
  (`/Game/GameOff2024/UI/UI_Transition.Start Level Loaded Transition` _ui_transition_widget))

(fn `StartLoadNewLevelTransition`
  (params (LevelName :type Name))
  (bind _ui_transition_widget (`self.UI Transition Widget`))
  (if (not (`Widget.IsInViewport` _ui_transition_widget))
    (`UserWidget.AddToViewport` _ui_transition_widget 0))
  (`/Game/GameOff2024/UI/UI_Transition.Start Load New Level Transition` _ui_transition_widget LevelName))