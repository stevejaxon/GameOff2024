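; BP_MainMenu_GM is the main menu game mode that brings up the menu when the level starts.
; Its construction script casts the game instance to BP_Main_GI and caches it.
; BeginPlay creates and displays the UI_MainMenu widget, tells the game instance to start the level-loaded transition, and then shows the mouse cursor.
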(event `self.ReceiveBeginPlay`
  (`|ExecutionSequence`
    (:`then_0`
      (bind _returnvalue (`|CreateWidget` "/Game/GameOff2024/UI/MainMenu/UI_MainMenu.UI_MainMenu_C"))
      (`UserWidget.AddToViewport` _returnvalue 0)
      (`/Game/GameOff2024/Core/GameModes/BP_Main_GI.StartLevelLoadedTransition` (`self.Main GI`)))
    (:`then_1`
      (set `PlayerController.bShowMouseCursor` true (`GameplayStatics.GetPlayerController` 0)))))

(fn `UserConstructionScript`
  (bind _asbp_main_gi (cast `/Game/GameOff2024/Core/GameModes/BP_Main_GI` (`GameplayStatics.GetGameInstance`)))
  (set `self.Main GI` _asbp_main_gi))